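; BP_Ball is the player's physics-driven ball, which attacks enemies and respawns at the PlayerStart.
; OnAttack calls the parent, locks input and freezes physics, then a looping timer strikes each TargetEnemies entry in turn, counting kills.
; Debug sphere and lines show the attack radius and hits, and control and physics return after the last target.
; Overlapping a KillZVolume or BP_Enemy teleports the ball back to the start.
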(event Custom|DrawLine
  (bind _counter (Variables|Default|GetCounter))
  (bind _targetenemies (Variables|Default|GetTargetEnemies))
  (bind _output (Utilities|Array|Get(acopy) _targetenemies _counter))
  ;[1 1 1] Нанесение урона противнику
  (Default|CallOnAttackEnemy _output)
  (Math|Integer|IncrementInt (Variables|Default|GetKillCount)
    (:%20%20
      (Rendering|Debug|DrawDebugLine (Transformation|GetActorLocation) (Transformation|GetActorLocation _output) "(R=1.000000,G=0.000000,B=0.000000,A=1.000000)" 0.1 0.0)
      (bind _result (Math|Integer|IncrementInt (Variables|Default|GetCounter))
        (:%20%20
          (if (== _result (Utilities|Array|Length (Variables|Default|GetTargetEnemies)))
            (Utilities|Time|ClearandInvalidateTimerbyHandle (Variables|Default|GetTimer))
            (Variables|Default|SetbIsInputDisabled false)
            (Physics|SetSimulatePhysics (Variables|Default|GetMeshComponent) true)))))))

(event EventOnAttack
  ;[1 1 1] Нанесение урона противнику
  (Variables|Default|SetbIsInputDisabled true)
  (Physics|SetSimulatePhysics (Variables|Default|GetMeshComponent) false)
  (|CallParentFunction)
  (Rendering|Debug|DrawDebugSphere (Transformation|GetActorLocation) (Variables|Default|GetAttackRadius) 12 "(R=1.000000,G=0.000000,B=0.000000,A=1.000000)" 0.1)
  (if (> (Utilities|Array|Length (Variables|Default|GetTargetEnemies)) 0)
    (Variables|Default|SetCounter 0)
    (bind _returnvalue (Utilities|Time|SetTimerbyEvent (delegate Custom|DrawLine) 0.1 true))
    (Variables|Default|SetTimer _returnvalue)
    (else
      (Variables|Default|SetbIsInputDisabled false)
      (Physics|SetSimulatePhysics (Variables|Default|GetMeshComponent) true))))

(event Collision|EventActorBeginOverlap
  (params (OtherActor :type Actor%20Object%20Reference))
  ;[1 1 1] При падении или столкновении с врагом игрок возвращается на стартовую позицию
  (Utilities|Casting|CastToKillZVolume OtherActor
    (:then
      _)
    (:CastFailed
      (Utilities|Casting|CastToBP_Enemy OtherActor)))
  (Physics|SetSimulatePhysics (Variables|Default|GetMeshComponent) false)
  (bind _returnvalue (Actor|GetActorOfClass "/Script/Engine.PlayerStart"))
  (Transformation|SetActorLocation (Transformation|GetActorLocation _returnvalue) false true)
  (Physics|SetSimulatePhysics (Variables|Default|GetMeshComponent) true))

(fn ConstructionScript)