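; Game mode that links ball attacks to enemy damage, handles level progression and ends the game.
; BeginPlay binds to the ball, enemies in each bridge's TriggerArray and the exit point, with exit binding and kill count loading inside the enemy loop.
; When the ball reaches the exit, Level 1 saves the kill count to the GameInstance and opens Level2.
; On Level 2, it pauses and shows the HUD end screen.
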(event Custom|OnAttackEnemy
  (params (Enemy :type Actor%20Object%20Reference))
  ;[1 1 1] Нанесение урона противнику
  (bind _asbp_enemy (Utilities|Casting|CastToBP_Enemy Enemy))
  (Class|Enemy|GetDamage _asbp_enemy))

(event Custom|EndGame
  ;[1 1 1] Окончание игры
  (Game|SetGamePaused true)
  (bind _asbp_hud (Utilities|Casting|CastToBP_HUD (HUD|GetHUD (Game|GetPlayerController 0))))
  (Default|ShowEndGameScreen _asbp_hud))

(event Custom|OnExitOverlap
  (params (Actor :type Actor%20Object%20Reference) (OtherActor :type Actor%20Object%20Reference))
  ;[1 1 1] При попадании игрока в зону выхода, либо загружаем следующий уровень, либо объявляем окончание игры
  (Utilities|Casting|CastToBP_Ball OtherActor)
  (bind _returnvalue (Game|GetCurrentLevelName true))
  (switch string _returnvalue
    (:Level1
      (CallFunction|SaveKillCount)
      (Game|OpenLevel(byName) "Level2"))
    (:Level2
      (CallFunction|EndGame))))

(event EventBeginPlay
  ;[1 1 1] Подпишемся на события нанесения и получения урона
  (bind _returnvalue (Actor|GetActorOfClass "/Game/Characters/BP_Ball.BP_Ball_C"))
  (EventDispatchers|BindEventtoOnAttackEnemy _returnvalue (EventDispatchers|CreateEvent :!event Custom|OnAttackEnemy))
  (bind _outactors (Actor|GetAllActorsOfClass "/Game/Environment/BP_Bridge.BP_Bridge_C"))
  (for _array_element _outactors
    (for _array_element_2 (Variables|/Script/RollingBall.Bridge|GetTriggerArray _array_element)
      (bind _asbp_enemy (Utilities|Casting|CastToBP_Enemy _array_element_2))
      (EventDispatchers|BindEventtoOnGetDamage _asbp_enemy (EventDispatchers|CreateEvent _array_element :!event CheckTrigger))
      (bind _returnvalue_2 (Actor|GetActorOfClass "/Game/Environment/BP_ExitPoint.BP_ExitPoint_C"))
      (Collision|BindEventtoOnActorBeginOverlap _returnvalue_2 (EventDispatchers|CreateEvent :!event Custom|OnExitOverlap))
      (CallFunction|LoadKillCount))))

(fn ConstructionScript)

(fn SaveKillCount
  (bind _asbp_ball (Utilities|Casting|CastToBP_Ball (Game|Player|GetPlayerPawn 0)))
  (bind _asbp_game_instance (Utilities|Casting|CastToBP_GameInstance (Game|GetGameInstance)))
  (Variables|/Game/BP_GameInstance.BP_GameInstance_C|SetKillCount _asbp_game_instance (Variables|/Game/Characters/BP_Ball.BP_Ball_C|GetKillCount _asbp_ball)))

(fn LoadKillCount
  (bind _asbp_game_instance (Utilities|Casting|CastToBP_GameInstance (Game|GetGameInstance)))
  (bind _asbp_ball (Utilities|Casting|CastToBP_Ball (Game|Player|GetPlayerPawn 0)))
  (Variables|/Game/Characters/BP_Ball.BP_Ball_C|SetKillCount _asbp_ball (Variables|/Game/BP_GameInstance.BP_GameInstance_C|GetKillCount _asbp_game_instance)))